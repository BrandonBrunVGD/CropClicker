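; BP_AddedItem is a short-lived floating indicator actor that shows an item image and a count, apparently for crops added to the player's items.
; On BeginPlay it applies CropImage to the Crop sprite and writes Number to the Quantity text, then destroys itself after a brief delay.
; Tick moves the actor upward by a fixed offset each frame without scaling by delta time, so its rise speed depends on frame rate.
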(event EventBeginPlay
  (Rendering|Components|Sprite|SetSprite (Variables|Default|GetCrop) (Variables|Default|GetCropImage))
  (Rendering|Components|TextRender|SetText (Variables|Default|GetQuantity) (Utilities|Text|ToText(Integer) (Variables|Default|GetNumber)))
  (Utilities|FlowControl|Delay 1.5)
  (Actor|DestroyActor))

(event Collision|EventActorBeginOverlap
  (params (OtherActor :type Actor%20Object%20Reference)))

(event EventTick
  (params (DeltaSeconds :type Float%20%28single-precision%29))
  (Transformation|AddActorWorldOffset "0.000000,0.000000,1.000000"))

(fn ConstructionScript)