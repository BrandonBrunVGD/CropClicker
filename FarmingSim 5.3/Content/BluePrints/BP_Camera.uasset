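; Player camera pawn for a crop-clicker game that pans sideways and holds coins, crop quantities and bug essence.
; Left clicks trace under the cursor to hit bugs or grow unlocked plots, with on-screen prompts for blocked crop clicks.
; Loads currencies, crops and per-plot state by PlotID on BeginPlay and saves on Destroyed.
; Includes a debug bug-spawn input and a capped away-earnings calculation that is never called.
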(event Custom|HandleBugHit
  (bind _returnvalue (Pawn|GetController))
  (bind _array (Utilities|Array|MakeArray "ObjectTypeQuery2"))
  (bind _asplayer_controller (Utilities|Casting|CastToPlayerController _returnvalue))
  (bind (_hitresult _returnvalue_2) (Class|PlayerController|GetHitResultUnderCursorforObjects _asplayer_controller _array true))
  (if (Variables|Default|GetCanClickBug)
    (if _returnvalue_2
      (bind _asbp_bug (Utilities|Casting|CastToBP_Bug (.HitActor (Collision|BreakHitResult _hitresult))))
      (Default|BugHit _asbp_bug))))

(event Custom|AddCoins_Event
  (params (Quantity :type Integer) (IsAddition :type Boolean))
  (if IsAddition
    (Variables|Default|SetCoins (+ (Variables|Default|GetCoins) Quantity))
    (else
      (Variables|Default|SetCoins (- (Variables|Default|GetCoins) Quantity)))))

(event Custom|HandleCropHit
  (bind _returnvalue (Pawn|GetController))
  (bind _array (Utilities|Array|MakeArray "ObjectTypeQuery2"))
  (bind _asplayer_controller (Utilities|Casting|CastToPlayerController _returnvalue))
  (bind (_hitresult _returnvalue_2) (Class|PlayerController|GetHitResultUnderCursorforObjects _asplayer_controller _array true))
  (if (Variables|Default|GetCanClickCrops)
    (if _returnvalue_2
      (bind _asbp_plot (Utilities|Casting|CastToBP_Plot (.HitActor (Collision|BreakHitResult _hitresult))))
      (if (not (Variables|/Game/BluePrints/BP_Plot.BP_Plot_C|GetPlotLocked _asbp_plot))
        (if (Utilities|Enum|Equal(Enum) (Variables|/Game/BluePrints/BP_Plot.BP_Plot_C|GetCropEnum _asbp_plot) "NewEnumerator3")
          (CallFunction|SpawnonScreenPromt "Oops! You Need To Select A Crop First!")
          (elif (Variables|/Game/BluePrints/BP_Plot.BP_Plot_C|GetBugActive _asbp_plot)
            (CallFunction|SpawnonScreenPromt "You Must Kill The Bug!")
            (else
              (Default|GrowCrop _asbp_plot))))))))

(event Custom|SpawnOnScreenPromt
  (params (text :type Text))
  (bind _onscreenpromt (Variables|Default|GetOnScreenPromt))
  (if (Variables|Default|GetTextPrompt)
    (Variables|/Game/BluePrints/UI/W_OnScreenPromt.W_OnScreenPromt_C|SetText _onscreenpromt text)
    (Widget|SetVisibility _onscreenpromt "HitTestInvisible")
    (Utilities|FlowControl|RetriggerableDelay 2.0)
    (Widget|SetVisibility _onscreenpromt "Collapsed")))

(event Custom|ChangeCropValues
  (params (Crop :type E_Crops%20Enum :default "NewEnumerator3") (Quantity :type Integer) (IsAddition :type Boolean))
  (bind _returnvalue (Math|Conversions|ToInteger(Byte) Crop))
  (bind _str_editable_crops_array (Variables|Default|GetSTR%20Editable%20Crops%20Array))
  (bind _output (Utilities|Array|Get(acopy) _str_editable_crops_array _returnvalue))
  (bind _quantity (Utilities|Struct|BreakSTR_EditableCropValues _output))
  (if IsAddition
    (Utilities|Struct|SetmembersinSTR_EditableCropValues _output (+ _quantity Quantity))
    (else
      (Utilities|Struct|SetmembersinSTR_EditableCropValues _output (+ _quantity (* Quantity -1))))))

(event Custom|HandleAwayCalculation
  (Variables|Default|SetTiimeElapsedInHours (/ (Math|Conversions|ToFloat(Integer) (- (.Minute (Math|DateTime|BreakDateTime (Math|DateTime|Now))) (.Minute (Math|DateTime|BreakDateTime (Variables|Default|GetPreviousTime))))) 6e+01))
  (for _array_element (Variables|Default|GetSTR%20Editable%20Crops%20Array)
    (if (> (.GatherMultuplier (Utilities|Struct|BreakSTR_EditableCropValues _array_element)) 0.0)
      (if (<= (Variables|Default|GetTiimeElapsedInHours) 6.0)
        (Utilities|Struct|SetmembersinSTR_EditableCropValues _array_element (+ (.Quantity (Utilities|Struct|BreakSTR_EditableCropValues _array_element)) (* (* (* (* (.GatherMultuplier (Utilities|Struct|BreakSTR_EditableCropValues _array_element)) (Variables|Default|GetCPS)) 6e+01) (Variables|Default|GetTiimeElapsedInHours)) 0.1)))
        (else
          (Utilities|Struct|SetmembersinSTR_EditableCropValues _array_element (+ (.Quantity (Utilities|Struct|BreakSTR_EditableCropValues _array_element)) (* (* (* (* (.GatherMultuplier (Utilities|Struct|BreakSTR_EditableCropValues _array_element)) (Variables|Default|GetCPS)) 6e+01) 6.0) 0.1)))))))
  (Development|PrintString (Utilities|String|Append "You Were Gone For: " (Utilities|String|ToString(Float) (Variables|Default|GetTiimeElapsedInHours)) " Hours!")))

(event EventBeginPlay
  (bind _returnvalue (UserInterface|CreateWidget "/Game/BluePrints/UI/W_OnScreenPromt.W_OnScreenPromt_C"))
  (bind _output_get (Variables|Default|SetOnScreenPromt _returnvalue))
  (UserInterface|Viewport|AddtoViewport _output_get 0)
  (Widget|SetVisibility _output_get "Collapsed")
  (CallFunction|FLoadGame (Variables|Default|GetPlayerSaves)))

(event Collision|EventActorBeginOverlap
  (params (OtherActor :type Actor%20Object%20Reference)))

(event EventTick
  (params (DeltaSeconds :type Float%20%28single-precision%29))
  (Transformation|AddActorWorldOffset (Math|Vector|MakeVector (* (stale Input|AxisEvents|InputAxisLeft/Right AxisValue) (Variables|Default|GetMovementSpeed)) 0.0 0.0)))

(event EventDestroyed
  (CallFunction|FSaveGame (Variables|Default|GetPlayerSaves)))

(event Input|ActionEvents|InputActionSpawnBug
  (params (Key :type Key%20Structure :default "None"))
  ;[1 1 1] DEBUG(lol) - Spawns bugs
  (:Pressed
    (bind _outactors (Actor|GetAllActorsOfClass "/Game/BluePrints/BP_Plot.BP_Plot_C"))
    (for _array_element _outactors
      (Default|SpawnBug _array_element))))

(event Input|AxisEvents|InputAxisLeft/Right
  (params (AxisValue :type Float%20%28single-precision%29)))

(event Input|MouseEvents|LeftMouseButton
  (params (Key :type Key%20Structure :default "None"))
  (:Pressed
    (CallFunction|HandleBugHit)
    (CallFunction|HandleCropHit)))

(fn ConstructionScript)

(fn FSaveGame
  (params (SlotName :type String))
  (bind _returnvalue (SaveGame|DoesSaveGameExist SlotName))
  (if _returnvalue
    (bind _returnvalue_2 (SaveGame|LoadGamefromSlot SlotName))
    (Variables|Default|SetSaveRef _returnvalue_2)
    (else
      (bind _returnvalue_3 (SaveGame|CreateSaveGameObject "/Game/BluePrints/BP_SaveGame.BP_SaveGame_C"))
      (bind _output_get (Variables|Default|SetSaveRef _returnvalue_3))))
  (bind _asbp_save_game (Utilities|Casting|CastToBP_SaveGame _output_get))
  (Variables|/Game/BluePrints/BP_SaveGame.BP_SaveGame_C|SetPreviousTime _asbp_save_game (Math|DateTime|Now))
  (Variables|/Game/BluePrints/BP_SaveGame.BP_SaveGame_C|SetSTR%20Editable%20Crops%20Array _asbp_save_game (Variables|Default|GetSTR%20Editable%20Crops%20Array))
  (Variables|/Game/BluePrints/BP_SaveGame.BP_SaveGame_C|SetCoins _asbp_save_game (Variables|Default|GetCoins))
  (Variables|/Game/BluePrints/BP_SaveGame.BP_SaveGame_C|SetBugEssence _asbp_save_game (Variables|Default|GetBugEssence))
  (bind _outactors (Actor|GetAllActorsOfClass "/Game/BluePrints/BP_Plot.BP_Plot_C"))
  (for _array_element _outactors
    (Utilities|Array|SetArrayElem (Variables|/Game/BluePrints/BP_SaveGame.BP_SaveGame_C|GetPlotLocked _asbp_save_game) (Variables|/Game/BluePrints/BP_Plot.BP_Plot_C|GetPlotID _array_element) (Variables|/Game/BluePrints/BP_Plot.BP_Plot_C|GetPlotLocked _array_element) true)
    (Utilities|Array|SetArrayElem (Variables|/Game/BluePrints/BP_SaveGame.BP_SaveGame_C|GetCropEnum _asbp_save_game) (Variables|/Game/BluePrints/BP_Plot.BP_Plot_C|GetPlotID _array_element) (Variables|/Game/BluePrints/BP_Plot.BP_Plot_C|GetCropEnum _array_element) true))
  (SaveGame|SaveGametoSlot (Variables|Default|GetSaveRef) SlotName))

(fn FLoadGame
  (params (SlotName :type String))
  (bind _returnvalue (SaveGame|DoesSaveGameExist SlotName))
  (if _returnvalue
    (bind _returnvalue_2 (SaveGame|LoadGamefromSlot SlotName))
    (bind _asbp_save_game (Utilities|Casting|CastToBP_SaveGame _returnvalue_2))
    (bind _outactors (Actor|GetAllActorsOfClass "/Game/BluePrints/BP_Plot.BP_Plot_C"))
    (for _array_element _outactors
      (Variables|/Game/BluePrints/BP_Plot.BP_Plot_C|SetPlotLocked _array_element (Utilities|Array|Get(acopy) (Variables|/Game/BluePrints/BP_SaveGame.BP_SaveGame_C|GetPlotLocked _asbp_save_game) (Variables|/Game/BluePrints/BP_Plot.BP_Plot_C|GetPlotID _array_element)))
      (Variables|/Game/BluePrints/BP_Plot.BP_Plot_C|SetCropEnum _array_element (Utilities|Array|Get(acopy) (Variables|/Game/BluePrints/BP_SaveGame.BP_SaveGame_C|GetCropEnum _asbp_save_game) (Variables|/Game/BluePrints/BP_Plot.BP_Plot_C|GetPlotID _array_element))))
    (Variables|Default|SetPreviousTime (Variables|/Game/BluePrints/BP_SaveGame.BP_SaveGame_C|GetPreviousTime _asbp_save_game))
    (Variables|Default|SetSTR%20Editable%20Crops%20Array (Variables|/Game/BluePrints/BP_SaveGame.BP_SaveGame_C|GetSTR%20Editable%20Crops%20Array _asbp_save_game))
    (Variables|Default|SetCoins (Variables|/Game/BluePrints/BP_SaveGame.BP_SaveGame_C|GetCoins _asbp_save_game))
    (Variables|Default|SetBugEssence (Variables|/Game/BluePrints/BP_SaveGame.BP_SaveGame_C|GetBugEssence _asbp_save_game))))