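; Farm plot for a clicker game that grows one crop, yields it to BP_Camera's capped inventory, and displays locked state.
; The paused crop flipbook stores growth: GrowCrop advances frames by click power, then gathers and resets once ripe.
; Tick polls lock visuals, ripeness and bug health.
; Ripe plots start a random-delay BP_Bug spawn, which blocks growing and gathering until its HP runs out, then awards Bug Essence.
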(event Custom|GrowCrop
  (bind _crop (Variables|Default|GetCrop))
  (if (not (Variables|Default|GetBugActive))
    (if (Variables|Default|GetCanGather)
      (CallFunction|Gather)
      (else
        (Class|PaperFlipbookComponent|SetPlaybackPositioninFrames _crop (+ (Class|PaperFlipbookComponent|GetPlaybackPositioninFrames _crop) (* 30 (Variables|/Game/BluePrints/BP_Camera.BP_Camera_C|GetClickPower (Variables|Default|GetAs%20BP%20Camera)))) false)))))

(event Custom|HandleLockedPlot
  (bind _lock (Variables|Default|GetLock))
  (bind _frame (Variables|Default|GetFrame))
  (if (Variables|Default|GetPlotLocked)
    (Rendering|SetVisibility _lock true false)
    (Sprite|SetSpriteColor _frame "(R=0.166667,G=0.166667,B=0.166667,A=1.000000)")
    (else
      (Rendering|SetVisibility _lock false false)
      (Sprite|SetSpriteColor _frame "(R=1.000000,G=1.000000,B=1.000000,A=1.000000)"))))

(event Custom|HandleBug
  (bind _reference_bp_bug (Variables|Default|GetReference%20BP_Bug))
  (bind _as_bp_camera (Variables|Default|GetAs%20BP%20Camera))
  (bind _ladybug (Variables|/Game/BluePrints/Bug/BP_Bug.BP_Bug_C|GetLadybug _reference_bp_bug))
  (bind _bugessencemultiplier (Variables|/Game/BluePrints/BP_Camera.BP_Camera_C|GetBugEssenceMultiplier _as_bp_camera))
  (bind _returnvalue (Transformation|GetWorldTransform _ladybug))
  (if (<= (Variables|/Game/BluePrints/Bug/BP_Bug.BP_Bug_C|GetHP _reference_bp_bug) 0.0)
    (Variables|Default|SetBugActive false)
    (Variables|/Game/BluePrints/BP_Camera.BP_Camera_C|SetBugEssence _as_bp_camera (+ (Variables|/Game/BluePrints/BP_Camera.BP_Camera_C|GetBugEssence _as_bp_camera) _bugessencemultiplier))
    (Game|SpawnActorfromClass "/Game/BluePrints/BP_AddedItem.BP_AddedItem_C" (Math|Transform|MakeTransform (Math|Vector|MakeVector (.x (.location _returnvalue)) (- (.y (.location _returnvalue)) 2.5e+02) (.z (.location _returnvalue))) "0.000000,180.000000,0.000000" "0.500000,0.500000,0.500000") "Undefined" "MultiplyWithRoot" 0 _bugessencemultiplier "/Game/BluePrints/BugEssence_Sprite.BugEssence_Sprite" 0)
    (Actor|DestroyActor _reference_bp_bug)))

(event Custom|HandleAddedItemPromt
  (params (Quantity :type Integer))
  (bind _frame (Variables|Default|GetFrame))
  (bind _returnvalue (Transformation|GetWorldTransform _frame))
  (if (Variables|/Game/BluePrints/BP_Camera.BP_Camera_C|GetCropPrompt (Variables|Default|GetAs%20BP%20Camera))
    (bind _returnvalue_2 (Utilities|GetDataTableRow "/Game/BluePrints/Crops/DT_Crops.DT_Crops" (Utilities|String|StringToName (Utilities|String|EnumtoString (Variables|Default|GetCropEnum))))
      (:then
        (Game|SpawnActorfromClass "/Game/BluePrints/BP_AddedItem.BP_AddedItem_C" (Math|Transform|MakeTransform (Math|Vector|MakeVector (.x (.location _returnvalue)) (- (.y (.location _returnvalue)) 2e+02) (.z (.location _returnvalue))) (.rotation _returnvalue) "0.500000,0.500000,0.500000") "Undefined" "MultiplyWithRoot" 0 Quantity (.Icon (Utilities|Struct|BreakSTR_Crops _returnvalue_2)) 0)))))

(event Custom|Gather
  (bind _cropenum (Variables|Default|GetCropEnum))
  (bind _as_bp_camera (Variables|Default|GetAs%20BP%20Camera))
  (bind _as_bp_camera_2 (Variables|Default|GetAs%20BP%20Camera))
  (bind _returnvalue (Math|Conversions|ToInteger(Byte) _cropenum))
  (bind _str_editable_crops_array (Variables|/Game/BluePrints/BP_Camera.BP_Camera_C|GetSTR%20Editable%20Crops%20Array _as_bp_camera))
  (bind _output (Utilities|Array|Get(acopy) _str_editable_crops_array _returnvalue))
  (bind (_quantity _gathermultuplier) (Utilities|Struct|BreakSTR_EditableCropValues _output))
  (bind _returnvalue_2 (Math|Float|Truncate _gathermultuplier))
  (if (< _quantity (Variables|/Game/BluePrints/BP_Camera.BP_Camera_C|GetMaxCrops _as_bp_camera))
    (Default|ChangeCropValues _as_bp_camera_2 _cropenum _returnvalue_2 true)
    (CallFunction|HandleAddedItemPromt _returnvalue_2)
    (Class|PaperFlipbookComponent|SetPlaybackPositioninFrames (Variables|Default|GetCrop) 0 false)
    (Variables|Default|SetCanGather false)
    (else
      (Default|SpawnonScreenPromt _as_bp_camera_2 (Utilities|Text|FormatText "Crop Limit For This Crop Has Been Reached!")))))

(event Custom|HandleFlipBook
  (bind _crop (Variables|Default|GetCrop))
  (bind _returnvalue (Utilities|GetDataTableRow "/Game/BluePrints/Crops/DT_Crops.DT_Crops" (Utilities|String|StringToName (Utilities|String|EnumtoString (Variables|Default|GetCropEnum))))
    (:then
      (Sprite|SetFlipbook _crop (.GrowingFB (Utilities|Struct|BreakSTR_Crops _returnvalue)))
      (Components|Timeline|SetPlayRate _crop 0.0))
    (:RowNotFound
      (Sprite|SetFlipbook _crop))))

(event Custom|SpawnBug
  (bind _frame (Variables|Default|GetFrame))
  (bind _returnvalue (Transformation|GetWorldTransform _frame))
  (bind _returnvalue_2 (Game|SpawnActorfromClass "/Game/BluePrints/Bug/BP_Bug.BP_Bug_C" (Math|Transform|MakeTransform (Math|Vector|MakeVector (.x (.location _returnvalue)) -4.6e+02 (.z (.location _returnvalue))) "0, 0, 0" "1.000000,1.000000,1.000000") "Undefined" "MultiplyWithRoot" 0 0))
  (Variables|Default|SetReference%20BP_Bug _returnvalue_2)
  (Variables|Default|SetBugActive true)
  (Default|SpawnonScreenPromt (Variables|Default|GetAs%20BP%20Camera) "A Bug Has Spawned, WOW!"))

(event Custom|HandleRandomBugSpawn
  (if (not (== (Variables|Default|GetCropEnum) 0))
    (if (not (Variables|Default|GetBugActive))
      (Utilities|FlowControl|Delay (Math|Random|RandomFloatinRange 3e+01 (* 6e+01 1.5)))
      (CallFunction|SpawnBug))))

(event EventBeginPlay
  (Utilities|FlowControl|Delay 0.2)
  (CallFunction|HandleFlipBook)
  (bind _asbp_camera (Utilities|Casting|CastToBP_Camera (Game|Player|GetPlayerPawn 0)))
  (Variables|Default|SetAs%20BP%20Camera _asbp_camera)
  (CallFunction|HandleLockedPlot))

(event EventTick
  (params (DeltaSeconds :type Float%20%28single-precision%29))
  (CallFunction|HandleLockedPlot)
  (if (Variables|Default|GetBugActive)
    (CallFunction|HandleBug)
    (elif (>= (Class|PaperFlipbookComponent|GetPlaybackPositioninFrames (Variables|Default|GetCrop)) 59)
      (Variables|Default|SetCanGather true)
      (CallFunction|HandleRandomBugSpawn))))

(fn ConstructionScript)